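; BP_FloorSpawnVolume is a box volume that keeps spawning BP_DropFloor actors at random points inside its bounds.
; BeginPlay starts a looping one-second timer that spawns each floor at a random location within the Box component's scaled extent.
; When destroyed, it destroys its directly attached actors, though this graph does not attach the spawned floors to it.
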(event `self.ReceiveBeginPlay`
  (`KismetSystemLibrary.K2_SetTimerDelegate` (delegate `SpawnActer`) 1.0 true))

(event `SpawnActer`
  (bind _box (`self.Box`))
  (`|SpawnActorFromClass` "/Game/VRLevel/DropObjects/BP_DropFloor.BP_DropFloor_C" (`KismetMathLibrary.Conv_VectorToTransform` (`KismetMathLibrary.RandomPointInBoundingBox` (`SceneComponent.K2_GetComponentLocation` _box) (`BoxComponent.GetScaledBoxExtent` _box))) "Undefined" "MultiplyWithRoot" null null))

(event `self.ReceiveDestroyed`
  (bind _output_get (set `self.Out FloorActors` (`self.GetAttachedActors` self true false)))
  (for _array_element _output_get
    (`self.K2_DestroyActor` _array_element)))

(fn `UserConstructionScript`)