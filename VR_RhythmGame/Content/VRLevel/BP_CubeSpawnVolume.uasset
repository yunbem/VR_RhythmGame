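; BP_CubeSpawnVolume is a VR level actor that spawns BP_DropCube actors at the world location of its Box component.
; The SpawnActer event performs the spawn, but the looping timer that would repeat it is disconnected, so nothing in this graph triggers it.
; When destroyed, the volume also destroys its directly attached actors, although the spawn code does not attach the cubes it creates.
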(event `self.ReceiveBeginPlay`)

(event `SpawnActer`
  (`|SpawnActorFromClass` "/Game/VRLevel/BP_DropCube.BP_DropCube_C" (`KismetMathLibrary.Conv_VectorToTransform` (`SceneComponent.K2_GetComponentLocation` (`self.Box`))) "Undefined" "MultiplyWithRoot" null null))

(event `self.ReceiveDestroyed`
  (bind _output_get (set `self.Out CubeActors` (`self.GetAttachedActors` self true false)))
  (for _array_element _output_get
    (`self.K2_DestroyActor` _array_element)))

(fn `UserConstructionScript`)