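; BP_DropFloor is a VR level actor that moves itself along a direction set by its Arrow component as soon as play begins.
; BeginPlay caches the start location, then a Timeline's Transform track, scaled by a large fixed distance, offsets the actor along the arrow's forward vector without sweeping.
; Overlap, Tick and the construction script are empty, and a leftover PrintString is unconnected.
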(event `self.ReceiveBeginPlay`
  (set `self.시작위치` (`self.K2_GetActorLocation`))
  (bind (_direction _transform) (`Timeline|Timeline`)
    (:`Update`
      (`self.K2_SetActorLocation` (+ (`self.시작위치`) (* (`SceneComponent.GetForwardVector` (`self.Arrow`)) (* _transform 10000.0)))))))

(event `self.ReceiveActorBeginOverlap`
  (params (OtherActor :type "Actor Object Reference")))

(event `self.ReceiveTick`
  (params (DeltaSeconds :type "Float (single-precision)")))

(fn `UserConstructionScript`)